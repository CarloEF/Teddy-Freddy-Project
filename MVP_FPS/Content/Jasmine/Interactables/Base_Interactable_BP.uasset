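; Base interactable actor that registers with the PlayerCharacter while it overlaps the InteractableArea and unregisters on exit.
; Overlap opens an input gate and creates or removes an on-screen prompt widget based on the player's HasButtonPrompt flag.
; The Interact input briefly flags the prompt as pressed, then enters the gate, which has nothing wired after it.
; SetHighlight toggles custom depth rendering on the mesh.
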(event OnComponentBeginOverlap(InteractableArea)
  (params (OverlappedComponent :type Primitive%20Component%20Object%20Reference) (OtherActor :type Actor%20Object%20Reference) (OtherComp :type Primitive%20Component%20Object%20Reference) (OtherBodyIndex :type Integer) (bFromSweep :type Boolean) (SweepResult :type Hit%20Result%20Structure%20%28by%20ref%29))
  ;[1 1 1] Player in Interactable Area
  (bind _asplayer_character (Utilities|Casting|CastToPlayerCharacter OtherActor))
  (Class|InteractBPI|RegisterInteractable(Message) _asplayer_character self)
  ;[1 1 1] Add & Remove Prompt From Screen
  (if (Variables|/Game/Carlo/FirstPersonBP/Blueprints/PlayerCharacter.PlayerCharacter_C|GetHasButtonPrompt _asplayer_character)
    (Utilities|FlowControl|Gate true) ; enters at Open
    (else
      (Variables|/Game/Carlo/FirstPersonBP/Blueprints/PlayerCharacter.PlayerCharacter_C|SetHasButtonPrompt _asplayer_character false)
      (bind _returnvalue (UserInterface|CreateWidget "/Game/Carlo/Widgets/InteractPromptWidget.InteractPromptWidget_C"))
      (UserInterface|Viewport|AddtoViewport _returnvalue 0)
      (Utilities|FlowControl|Gate true) ; enters at Open
    )))

(event OnComponentEndOverlap(InteractableArea)
  (params (OverlappedComponent :type Primitive%20Component%20Object%20Reference) (OtherActor :type Actor%20Object%20Reference) (OtherComp :type Primitive%20Component%20Object%20Reference) (OtherBodyIndex :type Integer))
  ;[1 1 1] Player in Interactable Area
  (bind _asplayer_character (Utilities|Casting|CastToPlayerCharacter OtherActor))
  (Class|InteractBPI|UnregisterInteractable(Message) _asplayer_character self)
  ;[1 1 1] Add & Remove Prompt From Screen
  (if (Variables|/Game/Carlo/FirstPersonBP/Blueprints/PlayerCharacter.PlayerCharacter_C|GetHasButtonPrompt _asplayer_character)
    (Widget|RemovefromParent (stale OnComponentBeginOverlap(InteractableArea) _returnvalue))
    (Utilities|FlowControl|Gate true) ; enters at Close
    (else
      (Utilities|FlowControl|Gate true) ; enters at Close
    )))

(event Input|ActionEvents|InputActionInteract
  (params (Key :type Key%20Structure :default "None"))
  (:Pressed
    (Variables|/Game/Carlo/Widgets/InteractPromptWidget.InteractPromptWidget_C|SetIsPressed (stale OnComponentBeginOverlap(InteractableArea) _returnvalue) true)
    (Utilities|FlowControl|Delay 0.3)
    (Variables|/Game/Carlo/Widgets/InteractPromptWidget.InteractPromptWidget_C|SetIsPressed (stale OnComponentBeginOverlap(InteractableArea) _returnvalue) false)
    (Utilities|FlowControl|Gate true)))

(fn ConstructionScript)

(fn SetHighlight
  (params (Highlight? :type Boolean))
  (Rendering|SetRenderCustomDepth (Variables|Default|GetInteractableMesh) Highlight?))