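; Small interactable door that swings open and closed on alternating player interactions, with an on-screen prompt widget.
; An overlap area registers the door with PlayerCharacter2, shows the prompt and opens a gate that lets Interaction through.
; A FlipFlop plays or reverses a timeline that drives the pivot's yaw.
; Timeline updates also spawn the door sound and, after a delay, clear the re-trigger lock and prompt pressed state.
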(event OnComponentBeginOverlap(InteractableArea)
  (params (OverlappedComponent :type Primitive%20Component%20Object%20Reference) (OtherActor :type Actor%20Object%20Reference) (OtherComp :type Primitive%20Component%20Object%20Reference) (OtherBodyIndex :type Integer) (bFromSweep :type Boolean) (SweepResult :type Hit%20Result%20Structure%20%28by%20ref%29))
  ;[1 1 1] Player in Interactable Area
  (bind _asplayer_character_2 (Utilities|Casting|CastToPlayerCharacter2 OtherActor))
  (Class|InteractBPI|RegisterInteractable(Message) _asplayer_character_2 self)
  ;[1 1 1] Add & Remove Prompt From Screen
  (Widget|SetVisibility (stale EventBeginPlay _returnvalue) "Visible")
  (Utilities|FlowControl|Gate true) ; enters at Open
)

(event OnComponentEndOverlap(InteractableArea)
  (params (OverlappedComponent :type Primitive%20Component%20Object%20Reference) (OtherActor :type Actor%20Object%20Reference) (OtherComp :type Primitive%20Component%20Object%20Reference) (OtherBodyIndex :type Integer))
  ;[1 1 1] Player in Interactable Area
  (bind _asplayer_character_2 (Utilities|Casting|CastToPlayerCharacter2 OtherActor))
  (Class|InteractBPI|UnregisterInteractable(Message) _asplayer_character_2 self)
  ;[1 1 1] Add & Remove Prompt From Screen
  (Widget|SetVisibility (stale EventBeginPlay _returnvalue) "Hidden")
  (Utilities|FlowControl|Gate true) ; enters at Close
)

(event EventBeginPlay
  (bind _returnvalue (UserInterface|CreateWidget "/Game/Carlo/Widgets/DoorPromptWidget.DoorPromptWidget_C"))
  (UserInterface|Viewport|AddtoViewport _returnvalue 0)
  (Widget|SetVisibility _returnvalue "Hidden"))

(event EventInteraction
  (params (Instigator :type Player%20Character%202%20Object%20Reference))
  (Utilities|FlowControl|Gate true
    (:Exit
      (Variables|/Game/Carlo/Widgets/DoorPromptWidget.DoorPromptWidget_C|SetIsPressed (stale EventBeginPlay _returnvalue) true)
      (if (not (Variables|Default|GetIsOpening))
        (Variables|Default|SetIsOpening true)
        (Utilities|FlowControl|FlipFlop
          (:A
            (bind _newtrack_0 (Timeline|Timeline_0 PlayFromStart)
              (:Update
                (Transformation|SetRelativeRotation (Variables|Default|GetPivot) (Math|Rotator|MakeRotator 0.0 0.0 _newtrack_0) false false)
                (Audio|SpawnSoundatLocation "/Game/Carlo/Interactables/Door_Opening_Sound_Effect.Door_Opening_Sound_Effect" (Transformation|GetActorLocation) "0, 0, 0" 1.0 1.0 0.0 0 0)
                (Utilities|FlowControl|Delay 1.0)
                (Variables|Default|SetIsOpening false)
                (Variables|/Game/Carlo/Widgets/DoorPromptWidget.DoorPromptWidget_C|SetIsPressed (stale EventBeginPlay _returnvalue) false))))
          (:B
            (Timeline|Timeline_0 ReverseFromEnd)))))))

(fn ConstructionScript
  (|CallParentFunction))