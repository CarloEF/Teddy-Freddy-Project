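; Keypad-locked exit door for Level 2 that loads the Victory level once opened.
; On BeginPlay it joins three codes from PersistentSettings into the required code; overlap registers it with the player, shows a prompt and gates interaction.
; Interacting opens a keypad widget and pauses the game.
; ConfirmCode either plays door and handle timelines with a creak, or flashes ERROR, briefly unpausing so its Delays can run.
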(event OnComponentBeginOverlap(InteractableArea)
  (params (OverlappedComponent :type Primitive%20Component%20Object%20Reference) (OtherActor :type Actor%20Object%20Reference) (OtherComp :type Primitive%20Component%20Object%20Reference) (OtherBodyIndex :type Integer) (bFromSweep :type Boolean) (SweepResult :type Hit%20Result%20Structure%20%28by%20ref%29))
  (bind _returnvalue (Game|GetPlayerController 0))
  (bind _self self)
  ;[1 1 1] Player in Interactable Area
  (bind _asplayer_character_2 (Utilities|Casting|CastToPlayerCharacter2 OtherActor))
  (Class|InteractBPI|RegisterInteractable(Message) _asplayer_character_2 _self)
  (Default|OverlappedKeypad _asplayer_character_2 _self)
  ;[1 1 1] Add & Remove Prompt From Screen
  (Widget|SetVisibility (stale EventBeginPlay _returnvalue) "Visible")
  (Utilities|FlowControl|Gate true) ; enters at Open
)

(event OnComponentEndOverlap(InteractableArea)
  (params (OverlappedComponent :type Primitive%20Component%20Object%20Reference) (OtherActor :type Actor%20Object%20Reference) (OtherComp :type Primitive%20Component%20Object%20Reference) (OtherBodyIndex :type Integer))
  (bind _returnvalue (Game|GetPlayerController 0))
  ;[1 1 1] Player in Interactable Area
  (bind _asplayer_character_2 (Utilities|Casting|CastToPlayerCharacter2 OtherActor))
  (Class|InteractBPI|UnregisterInteractable(Message) _asplayer_character_2 self)
  ;[1 1 1] Add & Remove Prompt From Screen
  (Widget|SetVisibility (stale EventBeginPlay _returnvalue) "Hidden")
  (Utilities|FlowControl|Gate true) ; enters at Close
)

(event Custom|MoveHandle
  ;[1 1 1] Moving Handle Animation
  (Utilities|FlowControl|FlipFlop
    (:A
      (bind _handlerotation (Timeline|Timeline_1 PlayFromStart)
        (:Update
          (Transformation|SetRelativeRotation (Variables|Default|GetHandle) (Math|Rotator|MakeRotator _handlerotation 0.0 0.0) false false))
        (:Finished
          (Utilities|FlowControl|Delay 1.0)
          (Game|OpenLevel(byName) "Victory"))))
    (:B
      (Timeline|Timeline_1 ReverseFromEnd))))

(event Custom|MoveDoor
  ;[1 1 1] Moving Door Animation
  (Utilities|FlowControl|FlipFlop
    (:A
      (bind _newtrack_0 (Timeline|Timeline_0 PlayFromStart)
        (:Update
          (Transformation|SetRelativeRotation (Variables|Default|GetInteractableMesh) (Math|Rotator|MakeRotator 0.0 0.0 _newtrack_0) false false))))
    (:B
      (Timeline|Timeline_0 ReverseFromEnd))))

(event Custom|ConfirmCode
  (params (CodeToConfirm :type String))
  (bind _returnvalue (Game|GetPlayerController 0))
  ;[1 1 1] Logic for pressing 'Enter' on Keypad UI
  (if (Utilities|Enum|Equal(Enum) CodeToConfirm (Variables|Default|GetRequiredCode))
    (Variables|/Script/Engine.PlayerController|SetbShowMouseCursor _returnvalue false)
    (Input|SetInputModeGameOnly _returnvalue)
    (Widget|RemovefromParent (stale EventInteraction _returnvalue_2))
    (if (not (Variables|Default|GetIsOpening))
      (Variables|Default|SetIsOpening true)
      (CallFunction|MoveDoor)
      (CallFunction|MoveHandle)
      (Audio|SpawnSoundatLocation "/Game/Carlo/CarloAssets/Sounds/DoorCreak.DoorCreak" (Transformation|GetActorLocation) "0, 0, 0" 1.0 1.0 0.0 0 0)
      (Game|SetGamePaused false))
    (else
      (Variables|/Game/Carlo/Widgets/InteractionWidgets/KeypadWidget2.KeypadWidget2_C|SetcurrentlyWrong (stale EventInteraction _returnvalue_2) true)
      (Variables|/Game/Carlo/Widgets/InteractionWidgets/KeypadWidget2.KeypadWidget2_C|SetCode (stale EventInteraction _returnvalue_2) "ERROR")
      (Appearance|SetColorandOpacity (Variables|/Game/Carlo/Widgets/InteractionWidgets/KeypadWidget2.KeypadWidget2_C|GetTextBlock_209 (stale EventInteraction _returnvalue_2)) (Variables|Default|GetErrorOpacity) :!class /Script/UMG.TextBlock)
      (Game|SetGamePaused false)
      (Utilities|FlowControl|Delay 0.25)
      (Variables|/Game/Carlo/Widgets/InteractionWidgets/KeypadWidget2.KeypadWidget2_C|SetCode (stale EventInteraction _returnvalue_2) "")
      (Utilities|FlowControl|Delay 0.1)
      (Variables|/Game/Carlo/Widgets/InteractionWidgets/KeypadWidget2.KeypadWidget2_C|SetCode (stale EventInteraction _returnvalue_2) "ERROR")
      (Utilities|FlowControl|Delay 0.25)
      (Variables|/Game/Carlo/Widgets/InteractionWidgets/KeypadWidget2.KeypadWidget2_C|SetCode (stale EventInteraction _returnvalue_2) "")
      (Game|SetGamePaused true)
      (Variables|/Game/Carlo/Widgets/InteractionWidgets/KeypadWidget2.KeypadWidget2_C|SetcurrentlyWrong (stale EventInteraction _returnvalue_2) false))))

(event EventBeginPlay
  ;[1 1 1] Creating initial hidden widgets + Setting initial Keypad Code
  (bind _returnvalue (UserInterface|CreateWidget "/Game/Carlo/Widgets/InteractionWidgets/DoorPromptWidget.DoorPromptWidget_C"))
  (UserInterface|Viewport|AddtoViewport _returnvalue 0)
  (Widget|SetVisibility _returnvalue "Hidden")
  (bind _aspersistent_settings (Utilities|Casting|CastToPersistentSettings (Game|GetGameInstance)))
  (bind _output_get (Variables|Default|SetRequiredCode (Utilities|String|Append (Utilities|String|Append (Utilities|String|ToString(Integer) (Variables|/Game/Carlo/PersistentSettings.PersistentSettings_C|GetCodeOne _aspersistent_settings)) (Utilities|String|ToString(Integer) (Variables|/Game/Carlo/PersistentSettings.PersistentSettings_C|GetCodeTwo _aspersistent_settings))) (Utilities|String|ToString(Integer) (Variables|/Game/Carlo/PersistentSettings.PersistentSettings_C|GetCodeThree _aspersistent_settings)))))
  (Development|PrintString _output_get))

(event EventInteraction
  (params (Instigator :type Player%20Character%202%20Object%20Reference))
  (bind _returnvalue (Game|GetPlayerController 0))
  (Utilities|FlowControl|Gate true
    (:Exit
      ;[1 1 1] Opens up Keypad Widget UI
      (Variables|/Game/Carlo/Widgets/InteractionWidgets/DoorPromptWidget.DoorPromptWidget_C|SetIsPressed (stale EventBeginPlay _returnvalue) true)
      (bind _returnvalue_2 (UserInterface|CreateWidget "/Game/Carlo/Widgets/InteractionWidgets/KeypadWidget2.KeypadWidget2_C"))
      (UserInterface|Viewport|AddtoViewport _returnvalue_2 0)
      (Variables|/Script/Engine.PlayerController|SetbShowMouseCursor _returnvalue true)
      (Input|SetInputModeUIOnly _returnvalue 0 "DoNotLock")
      (Game|SetGamePaused true))))

(fn ConstructionScript
  (|CallParentFunction))

(fn NewFunction0)