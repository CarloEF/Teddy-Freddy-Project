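; BP_NoPromptNarrowDoor is an interactable door that toggles open and closed when the player interacts within range.
; Overlapping InteractableArea registers it with PlayerCharacter2 and opens a Gate that lets Interaction through.
; Each use plays a creak sound and uses FlipFlops to alternate two timelines forward and backward, rotating the mesh's yaw and the handle's roll.
; An IsOpening flag blocks retriggering, cleared by a one-second Delay from the handle timeline's update.
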(event OnComponentBeginOverlap(InteractableArea)
  (params (OverlappedComponent :type Primitive%20Component%20Object%20Reference) (OtherActor :type Actor%20Object%20Reference) (OtherComp :type Primitive%20Component%20Object%20Reference) (OtherBodyIndex :type Integer) (bFromSweep :type Boolean) (SweepResult :type Hit%20Result%20Structure%20%28by%20ref%29))
  ;[1 1 1] Player in Interactable Area
  (bind _asplayer_character_2 (Utilities|Casting|CastToPlayerCharacter2 OtherActor))
  (Class|InteractBPI|RegisterInteractable(Message) _asplayer_character_2 self)
  (Utilities|FlowControl|Gate true) ; enters at Open
)

(event OnComponentEndOverlap(InteractableArea)
  (params (OverlappedComponent :type Primitive%20Component%20Object%20Reference) (OtherActor :type Actor%20Object%20Reference) (OtherComp :type Primitive%20Component%20Object%20Reference) (OtherBodyIndex :type Integer))
  ;[1 1 1] Player in Interactable Area
  (bind _asplayer_character_2 (Utilities|Casting|CastToPlayerCharacter2 OtherActor))
  (Class|InteractBPI|UnregisterInteractable(Message) _asplayer_character_2 self)
  (Utilities|FlowControl|Gate true) ; enters at Close
)

(event Custom|MoveHandle
  (Utilities|FlowControl|FlipFlop
    (:A
      (bind _handlerotation (Timeline|Timeline_1 ReverseFromEnd)
        (:Update
          (Transformation|SetRelativeRotation (Variables|Default|GetHandle) (Math|Rotator|MakeRotator _handlerotation 0.0 0.0) false false)
          (Utilities|FlowControl|Delay 1.0)
          (Variables|Default|SetIsOpening false))))
    (:B
      (Timeline|Timeline_1 PlayFromStart))))

(event Custom|MoveDoor
  (Utilities|FlowControl|FlipFlop
    (:A
      (bind _newtrack_0 (Timeline|Timeline_0 PlayFromStart)
        (:Update
          (Transformation|SetRelativeRotation (Variables|Default|GetInteractableMesh) (Math|Rotator|MakeRotator 0.0 0.0 _newtrack_0) false false))))
    (:B
      (Timeline|Timeline_0 ReverseFromEnd))))

(event EventInteraction
  (params (Instigator :type Player%20Character%202%20Object%20Reference))
  (Utilities|FlowControl|Gate true
    (:Exit
      (if (not (Variables|Default|GetIsOpening))
        (Variables|Default|SetIsOpening true)
        (CallFunction|MoveDoor)
        (CallFunction|MoveHandle)
        (Audio|SpawnSoundatLocation "/Game/Carlo/CarloAssets/Sounds/DoorCreak.DoorCreak" (Transformation|GetActorLocation) "0, 0, 0" 1.0 1.0 0.0 0 0)))))

(fn ConstructionScript
  (|CallParentFunction))

(fn NewFunction0)