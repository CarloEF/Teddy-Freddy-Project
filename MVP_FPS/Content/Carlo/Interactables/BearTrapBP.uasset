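; Bear trap interactable that traps the player character when they walk into it.
; On actor overlap while enabled, it plays a sound, then flags the player character as trapped and passes itself to their trap handler.
; It plays the closing animation on its mesh, then disables itself and re-enables after a short delay.
; The sound fires before the player cast, so any overlapping actor triggers it.
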(event Collision|EventActorBeginOverlap
  (params (OtherActor :type Actor%20Object%20Reference))
  ;[1 1 1] Player in BearTrap Trigger Radius
  (if (Variables|Default|GetEnabled)
    (Audio|PlaySoundatLocation "/Game/Carlo/CarloAssets/Sounds/BearTrapSound2.BearTrapSound2" (Transformation|GetActorLocation) "0, 0, 0" 1.0 1.0 0.0 0 0 0)
    (bind _asplayer_character_2 (Utilities|Casting|CastToPlayerCharacter2 OtherActor))
    (Variables|/Game/Carlo/Character/PlayerCharacter2.PlayerCharacter2_C|SetisTrapped _asplayer_character_2 true)
    (Default|TrapTriggered _asplayer_character_2 self)
    (Components|Animation|PlayAnimation (Variables|Default|GetTrapMesh) "/Game/Jim/bear_trap/trap_closetrap_close_Anim.trap_closetrap_close_Anim" false)
    (Development|PrintString "Trap Triggered!")
    (Variables|Default|SetEnabled false)
    (Utilities|FlowControl|Delay 5.0)
    (Variables|Default|SetEnabled true)))

(fn ConstructionScript)