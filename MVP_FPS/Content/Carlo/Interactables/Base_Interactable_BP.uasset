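; Base interactable actor that shows an interaction prompt while its area is overlapped and destroys itself on interaction.
; Overlap events register or unregister it with PlayerCharacter2, toggle the prompt widget created on BeginPlay, and open or close a gate.
; Interact input briefly flags the prompt as pressed, then, if the gate is open, removes the widget and actor.
; SetHighlight toggles the mesh's custom depth rendering for highlighting.
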(event OnComponentBeginOverlap(InteractableArea)
  (params (OverlappedComponent :type Primitive%20Component%20Object%20Reference) (OtherActor :type Actor%20Object%20Reference) (OtherComp :type Primitive%20Component%20Object%20Reference) (OtherBodyIndex :type Integer) (bFromSweep :type Boolean) (SweepResult :type Hit%20Result%20Structure%20%28by%20ref%29))
  ;[1 1 1] Player in Interactable Area
  (bind _asplayer_character_2 (Utilities|Casting|CastToPlayerCharacter2 (Game|GetPlayerCharacter 0)))
  (Class|InteractBPI|RegisterInteractable(Message) _asplayer_character_2 self)
  ;[1 1 1] Add & Remove Prompt From Screen
  (Widget|SetVisibility (stale EventBeginPlay _returnvalue) "Visible")
  ;[1 1 1] Logic for Interactions
  (Utilities|FlowControl|Gate true) ; enters at Open
)

(event OnComponentEndOverlap(InteractableArea)
  (params (OverlappedComponent :type Primitive%20Component%20Object%20Reference) (OtherActor :type Actor%20Object%20Reference) (OtherComp :type Primitive%20Component%20Object%20Reference) (OtherBodyIndex :type Integer))
  ;[1 1 1] Player in Interactable Area
  (bind _asplayer_character_2 (Utilities|Casting|CastToPlayerCharacter2 (Game|GetPlayerCharacter 0)))
  (Class|InteractBPI|UnregisterInteractable(Message) _asplayer_character_2 self)
  ;[1 1 1] Add & Remove Prompt From Screen
  (Widget|SetVisibility (stale EventBeginPlay _returnvalue) "Hidden")
  ;[1 1 1] Logic for Interactions
  (Utilities|FlowControl|Gate true) ; enters at Close
)

(event EventBeginPlay
  ;[1 1 1] Creating Initial Hidden Widgets
  (bind _returnvalue (UserInterface|CreateWidget "/Game/Carlo/Widgets/InteractionWidgets/InteractPromptWidget.InteractPromptWidget_C"))
  (UserInterface|Viewport|AddtoViewport _returnvalue 0)
  (Widget|SetVisibility _returnvalue "Hidden"))

(event Input|ActionEvents|InputActionInteract
  (params (Key :type Key%20Structure :default "None"))
  ;[1 1 1] Logic for Interactions
  (:Pressed
    (Variables|/Game/Carlo/Widgets/InteractionWidgets/InteractPromptWidget.InteractPromptWidget_C|SetIsPressed (stale EventBeginPlay _returnvalue) true)
    (Utilities|FlowControl|Delay 0.3)
    (Variables|/Game/Carlo/Widgets/InteractionWidgets/InteractPromptWidget.InteractPromptWidget_C|SetIsPressed (stale EventBeginPlay _returnvalue) false)
    (Utilities|FlowControl|Gate true
      (:Exit
        (Widget|RemovefromParent (stale EventBeginPlay _returnvalue))
        (Actor|DestroyActor)))))

(fn ConstructionScript)

(fn SetHighlight
  (params (Highlight? :type Boolean))
  (Rendering|SetRenderCustomDepth (Variables|Default|GetInteractableMesh) Highlight?))