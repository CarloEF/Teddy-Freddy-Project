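; BP_Paper2 is an interactable paper note that the player picks up.
; On interaction it sends its item info to the instigator's pickup message and sets the HasFirstNote flag on PlayerCharacter2.
; It then shows the SecondNoteWidget, calls the FoundNote dispatcher and destroys itself.
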(event EventInteraction
  (params (Instigator :type Player%20Character%202%20Object%20Reference))
  ;[1 1 1] Interaction
  (Class|InteractBPI|Pickup(Message) Instigator (Variables|Default|GetItemInfo))
  (bind _asplayer_character_2 (Utilities|Casting|CastToPlayerCharacter2 (Game|GetPlayerCharacter 0)))
  (Variables|/Game/Carlo/Character/PlayerCharacter2.PlayerCharacter2_C|SetHasFirstNote _asplayer_character_2 true)
  (bind _returnvalue (UserInterface|CreateWidget "/Game/Carlo/Widgets/PersistentScreenWidgets/SecondNoteWidget.SecondNoteWidget_C"))
  (UserInterface|Viewport|AddtoViewport _returnvalue 0)
  (Default|CallFoundNote)
  (Actor|DestroyActor))

(fn ConstructionScript
  (|CallParentFunction))