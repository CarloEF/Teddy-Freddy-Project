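; Base interactable item that the player picks up, removing it from the world.
; On Interaction it passes its ItemInfo to the instigator through PickupMessage, sets HasKey on player 0's PlayerCharacter2, then destroys itself.
; HasKey is set regardless of item type, and the destroy only happens if that cast succeeds.
; A construction-script node that would write the item's own class into ItemInfo is left unconnected.
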(event EventInteraction
  (params (Instigator :type Player%20Character%202%20Object%20Reference))
  (Class|InteractBPI|Pickup(Message) Instigator (Variables|Default|GetItemInfo))
  (bind _asplayer_character_2 (Utilities|Casting|CastToPlayerCharacter2 (Game|GetPlayerCharacter 0)))
  (Variables|/Game/Carlo/FirstPersonBP/Blueprints/PlayerCharacter2.PlayerCharacter2_C|SetHasKey _asplayer_character_2 true)
  (Actor|DestroyActor))

(fn ConstructionScript
  (|CallParentFunction))